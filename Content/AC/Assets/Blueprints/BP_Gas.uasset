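; BP_Gas is a gas hazard that deals periodic damage to the player while they are inside its sphere trigger.
; Overlap begin caches the Core_PlayerCharacter1 and starts a looping timer that applies DamageDealt every DamageInterval.
; Overlap end by the player pauses that timer through its stored handle rather than clearing it.
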(event OnComponentBeginOverlap(Sphere)
  (params (OverlappedComponent :type Primitive%20Component%20Object%20Reference) (OtherActor :type Actor%20Object%20Reference) (OtherComp :type Primitive%20Component%20Object%20Reference) (OtherBodyIndex :type Integer) (bFromSweep :type Boolean) (SweepResult :type Hit%20Result%20Structure%20%28by%20ref%29))
  (bind _ascore_player_character_1 (Utilities|Casting|CastToCore_PlayerCharacter1 OtherActor))
  (bind _returnvalue (Utilities|Time|SetTimerbyEvent (delegate Custom|OnPlayerInsideTrigger) (Variables|Editablevalues|GetDamageInterval) true))
  (Variables|Default|SetTimerDamageDealer _returnvalue))

(event OnComponentEndOverlap(Sphere)
  (params (OverlappedComponent :type Primitive%20Component%20Object%20Reference) (OtherActor :type Actor%20Object%20Reference) (OtherComp :type Primitive%20Component%20Object%20Reference) (OtherBodyIndex :type Integer))
  (Utilities|Casting|CastToCore_PlayerCharacter1 OtherActor)
  (Utilities|Time|PauseTimerbyHandle (Variables|Default|GetTimerDamageDealer)))

(event Custom|OnPlayerInsideTrigger
  (Game|Damage|ApplyDamage (stale OnComponentBeginOverlap(Sphere) _ascore_player_character_1) (Variables|Editablevalues|GetDamageDealt) 0 0))

(fn ConstructionScript)