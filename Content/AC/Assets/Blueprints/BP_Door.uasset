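; BP_Door is an interactive door that the player opens with the E key while standing near it.
; Overlapping the Trigger with a Core_PlayerCharacter1 enables input on the door for player 0, and leaving disables it.
; Pressing E plays the DoorController timeline, which lerps SMDoor's relative location from StartPos to EndPos.
; The timeline only plays forward, with no logic to close the door.
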(event OnComponentBeginOverlap(Trigger)
  (params (OverlappedComponent :type Primitive%20Component%20Object%20Reference) (OtherActor :type Actor%20Object%20Reference) (OtherComp :type Primitive%20Component%20Object%20Reference) (OtherBodyIndex :type Integer) (bFromSweep :type Boolean) (SweepResult :type Hit%20Result%20Structure%20%28by%20ref%29))
  ;[1 1 1] Enable inputs
  (Utilities|Casting|CastToCore_PlayerCharacter1 OtherActor)
  (Input|EnableInput (Game|GetPlayerController 0)))

(event OnComponentEndOverlap(Trigger)
  (params (OverlappedComponent :type Primitive%20Component%20Object%20Reference) (OtherActor :type Actor%20Object%20Reference) (OtherComp :type Primitive%20Component%20Object%20Reference) (OtherBodyIndex :type Integer))
  ;[1 1 1] Enable inputs
  (Utilities|Casting|CastToCore_PlayerCharacter1 OtherActor)
  (Input|DisableInput (Game|GetPlayerController 0)))

(event Input|KeyboardEvents|E
  (params (Key :type Key%20Structure))
  ;[1 1 1] Door: lerp open when nearby
  (:Pressed
    (bind _newtrack_0 (Timeline|DoorController Play)
      (:Update
        (Transformation|SetRelativeLocation (Variables|Default|GetSM_Door) (Math|Vector|Lerp(Vector) (Variables|Default|GetStartPos) (Variables|Default|GetEndPos) _newtrack_0) false false)))))

(fn ConstructionScript)