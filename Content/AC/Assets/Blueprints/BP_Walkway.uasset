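; BP_Walkway is a button-operated walkway that rotates in 90-degree yaw steps when the player presses E inside its trigger.
; Trigger overlaps with the player character enable and disable input on the actor.
; E or RotateWalkway passes a DoOnce gate to play a timeline that lerps the mesh rotation, then advances the start and end angles and reopens the gate.
; Older GameInstance button-flag logic remains but never runs.
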(event OnComponentBeginOverlap(Trigger)
  (params (OverlappedComponent :type Primitive%20Component%20Object%20Reference) (OtherActor :type Actor%20Object%20Reference) (OtherComp :type Primitive%20Component%20Object%20Reference) (OtherBodyIndex :type Integer) (bFromSweep :type Boolean) (SweepResult :type Hit%20Result%20Structure%20%28by%20ref%29))
  ;[1 1 1] Enable input for button
  (Utilities|Casting|CastToCore_PlayerCharacter1 OtherActor)
  (Input|EnableInput (Game|GetPlayerController 0)))

(event OnComponentEndOverlap(Trigger)
  (params (OverlappedComponent :type Primitive%20Component%20Object%20Reference) (OtherActor :type Actor%20Object%20Reference) (OtherComp :type Primitive%20Component%20Object%20Reference) (OtherBodyIndex :type Integer))
  ;[1 1 1] Enable input for button
  (Utilities|Casting|CastToCore_PlayerCharacter1 OtherActor)
  (Input|DisableInput (Game|GetPlayerController 0)))

(event Custom|Rotate%20Walkway
  ;[1 1 1] Rotate walkway 90*
  (Utilities|FlowControl|DoOnce false :!label _label
    (:Completed
      (Components|Timeline|SetPlayRate (Variables|Default|Getrotation) 0.2)
      (bind _newtrack_0 (Timeline|rotation PlayFromStart)
        (:Update
          (Transformation|SetRelativeRotation (Variables|Default|GetSM_CS_Walkway) (Math|Rotator|Lerp(Rotator) (Variables|Default|GetStartPos) (Variables|Default|GetEndPos) _newtrack_0) false false))
        (:Finished
          (Variables|Default|SetStartPos (Variables|Default|GetEndPos))
          (Variables|Default|SetEndPos (Math|Rotator|MakeRotator 0.0 0.0 (+ (.yaw (Variables|Default|GetStartPos)) 9e+01)))
          (goto _label Reset))))))

(event Input|KeyboardEvents|E
  (params (Key :type Key%20Structure))
  ;[1 1 1] Rotate walkway 90*
  (:Pressed
    (Development|PrintString "*Click*")
    (Utilities|FlowControl|DoOnce false :!label _label
      (:Completed
        (Components|Timeline|SetPlayRate (Variables|Default|Getrotation) 0.2)
        (bind _newtrack_0 (Timeline|rotation PlayFromStart)
          (:Update
            (Transformation|SetRelativeRotation (Variables|Default|GetSM_CS_Walkway) (Math|Rotator|Lerp(Rotator) (Variables|Default|GetStartPos) (Variables|Default|GetEndPos) _newtrack_0) false false))
          (:Finished
            (Variables|Default|SetStartPos (Variables|Default|GetEndPos))
            (Variables|Default|SetEndPos (Math|Rotator|MakeRotator 0.0 0.0 (+ (.yaw (Variables|Default|GetStartPos)) 9e+01)))
            (goto _label Reset)))))))

(fn ConstructionScript)