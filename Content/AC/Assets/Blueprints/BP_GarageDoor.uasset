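; BP_GarageDoor is a garage door that opens when the player is nearby, once a control panel has been activated.
; Trigger overlap checks the HasActivatedControlPanel flag on Core_GameInstance, printing an "activated somewhere else" message if it is unset.
; If set, the DoorController timeline lerps the door mesh's relative location from StartPos to EndPos.
; The player leaving the trigger reverses the timeline.
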(event OnComponentBeginOverlap(Trigger)
  (params (OverlappedComponent :type Primitive%20Component%20Object%20Reference) (OtherActor :type Actor%20Object%20Reference) (OtherComp :type Primitive%20Component%20Object%20Reference) (OtherBodyIndex :type Integer) (bFromSweep :type Boolean) (SweepResult :type Hit%20Result%20Structure%20%28by%20ref%29))
  ;[1 1 1] Open when nearby if computer has been activated
  (Utilities|Casting|CastToCore_PlayerCharacter1 OtherActor)
  (bind _ascore_game_instance (Utilities|Casting|CastToCore_GameInstance (Game|GetGameInstance)))
  (if (Variables|/Game/AC/Core/Framework/Core_GameInstance.Core_GameInstance_C|GetbHasActivatedControlPanel _ascore_game_instance)
    (bind _alpha (Timeline|DoorController Play)
      (:Update
        (Transformation|SetRelativeLocation (Variables|Default|GetSM_CS_GarageDoor) (Math|Vector|Lerp(Vector) (Variables|Default|GetStartPos) (Variables|Default|GetEndPos) _alpha) false false)))
    (else
      (Development|PrintString "This door is activated somewhere else" true true "(R=1.000000,G=0.000000,B=0.927672,A=1.000000)"))))

(event OnComponentEndOverlap(Trigger)
  (params (OverlappedComponent :type Primitive%20Component%20Object%20Reference) (OtherActor :type Actor%20Object%20Reference) (OtherComp :type Primitive%20Component%20Object%20Reference) (OtherBodyIndex :type Integer))
  ;[1 1 1] Open when nearby if computer has been activated
  (Utilities|Casting|CastToCore_PlayerCharacter1 OtherActor)
  (bind _alpha (Timeline|DoorController Reverse)
    (:Update
      (Transformation|SetRelativeLocation (Variables|Default|GetSM_CS_GarageDoor) (Math|Vector|Lerp(Vector) (Variables|Default|GetStartPos) (Variables|Default|GetEndPos) _alpha) false false))))

(fn ConstructionScript)